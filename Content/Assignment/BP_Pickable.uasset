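; BP_Pickable is a configurable pickup actor that the player collects by overlapping its box.
; On overlap by the player character, it plays a sound, spawns a particle effect, increments the matching resource on the GS_IntroState game state, then destroys itself.
; The construction script applies the mesh and material variables to the Sphere component, so each placed pickup can differ in look, resource type and amount.
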(event `self.Box.OnComponentBeginOverlap`
  (params (OverlappedComponent :type "PrimitiveComponent Object Reference") (OtherActor :type "Actor Object Reference") (OtherComp :type "PrimitiveComponent Object Reference") (OtherBodyIndex :type Integer) (bFromSweep :type Boolean) (SweepResult :type "HitResult Structure (by ref)"))
  (if (== OtherActor (`GameplayStatics.GetPlayerCharacter` 0))
    (`|ExecutionSequence`
      (:`then_1`
        (`GameplayStatics.SpawnSoundAtLocation` (`self.Pickup_Sound`) (`self.K2_GetActorLocation` self) (struct) 1.0 1.0 0.0 null null))
      (:`then_2`
        (`GameplayStatics.SpawnEmitterAtLocation` (`self.Pickup_Particle`) (`self.K2_GetActorLocation` self) (struct) (0.8 0.8 0.8)))
      (:`then_3`
        (`/Game/Assignment/GS_IntroState.Increment_Resource` (cast `/Game/Assignment/GS_IntroState` (`GameplayStatics.GetGameState`) :!pure true) (`self.Amount_Collected`) (`self.Pickable_Type`)))
      (:`then_4`
        (`self.K2_DestroyActor`)))))

(fn `UserConstructionScript`
  (`StaticMeshComponent.SetStaticMesh` (`self.Sphere`) (`self.Static_Mesh`))
  (`PrimitiveComponent.SetMaterial` (`self.Sphere`) 0 (`self.Material`)))